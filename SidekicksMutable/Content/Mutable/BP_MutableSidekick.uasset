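; BP_MutableSidekick is a controllable sidekick with camera controls for viewing it and a mesh morph hook for its jaw.
; Enhanced Input events rotate via controller yaw and pitch, zoom by changing spring arm length, and pan by shifting the socket offset along the arm's right and up axes.
; UpdateJawOpen prints the mesh's current "jawOpen" morph weight, then sets it from the JawOpen variable.
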(event Input|EnhancedActionEvents|EnhancedInputActionIA_RotateCharacter
  (params (ActionValue :type Vector%202D%20Structure) (ElapsedSeconds :type Float%20%28double-precision%29) (TriggeredSeconds :type Float%20%28double-precision%29) (InputAction :type Input%20Action%20Object%20Reference :default "/Game/Inputs/IA/IA_RotateCharacter.IA_RotateCharacter"))
  ;[0.15 0.15 0.15 0.5] Controls
  (Pawn|Input|AddControllerYawInput (.x ActionValue))
  (Pawn|Input|AddControllerPitchInput (.y ActionValue)))

(event Input|EnhancedActionEvents|EnhancedInputActionIA_ZoomControl
  (params (ActionValue :type Float%20%28double-precision%29) (ElapsedSeconds :type Float%20%28double-precision%29) (TriggeredSeconds :type Float%20%28double-precision%29) (InputAction :type Input%20Action%20Object%20Reference :default "/Game/Inputs/IA/IA_ZoomControl.IA_ZoomControl"))
  (bind _springarm (Variables|Default|GetSpringArm))
  ;[0.15 0.15 0.15 0.5] Controls
  (Variables|/Script/Engine.SpringArmComponent|SetTargetArmLength _springarm (+ (Variables|/Script/Engine.SpringArmComponent|GetTargetArmLength _springarm) (* ActionValue (Math|Float|MakeLiteralFloat 3e+01)))))

(event Input|EnhancedActionEvents|EnhancedInputActionIA_Pan
  (params (ActionValue :type Vector%202D%20Structure) (ElapsedSeconds :type Float%20%28double-precision%29) (TriggeredSeconds :type Float%20%28double-precision%29) (InputAction :type Input%20Action%20Object%20Reference :default "/Game/Inputs/IA/IA_Pan.IA_Pan"))
  (bind _springarm (Variables|Default|GetSpringArm))
  (bind _returnvalue (Class|SpringArmComponent|GetTargetRotation _springarm))
  ;[0.15 0.15 0.15 0.5] Controls
  (Variables|/Script/Engine.SpringArmComponent|SetSocketOffset (Variables|Default|GetSpringArm) (+ (Variables|/Script/Engine.SpringArmComponent|GetSocketOffset (Variables|Default|GetSpringArm)) (Math|Vector|UnrotateVector (* (+ (* (Math|Vector|GetRightVector _returnvalue) (.x ActionValue)) (* (Math|Vector|GetUpVector _returnvalue) (.y ActionValue))) 1e+01) _returnvalue))))

(fn ConstructionScript)

(fn UpdateJawOpen
  (bind _mesh (Variables|Character|GetMesh))
  (Development|PrintText (Utilities|Text|FormatText "Mesh: {A}" (Class|SkeletalMeshComponent|GetMorphTarget _mesh "jawOpen")))
  (Components|SkeletalMesh|SetMorphTarget _mesh "jawOpen" (Variables|Morphs|GetJawOpen) true))