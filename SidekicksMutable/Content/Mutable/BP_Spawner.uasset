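; Spawner actor Blueprint meant to populate the area around it with Mutable-customized BP_MutableSidekick characters, but its spawn logic is disconnected and BeginPlay does nothing.
; The unwired logic generates population instances from PopRef and spawns a sidekick for each at a random navigable point nearby, with random yaw and scale.
; Each sidekick receives its Customizable Object instance and updates its skeletal mesh asynchronously.
; A second orphaned branch spawns at random offsets and prints a failure message.
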(event EventBeginPlay)

(fn ConstructionScript)